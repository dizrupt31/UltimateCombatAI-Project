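; BPC_Agression is a Blueprint component that stores an aggression value.
; AddAgression and SubtractAgression adjust CurrentAgression and clamp it between MinAgression and MaxAgression, while GetAgression returns the current value.
; The event graph has no active logic, so the value changes here only through those function calls.
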(event EventBeginPlay)

(event EventTick
  (params (DeltaSeconds :type Float%20%28single-precision%29)))

(fn GetAgression
  (return (Variables|Default|GetCurrentAgression)))

(fn AddAgression
  (params (AddedAgression :type Float%20%28double-precision%29))
  (Variables|Default|SetCurrentAgression (Math|Float|Clamp(Float) (+ AddedAgression (Variables|Default|GetCurrentAgression)) (Variables|Default|GetMinAgression) (Variables|Default|GetMaxAgression)))
  (return))

(fn SubtractAgression
  (params (SubtractedAgression :type Float%20%28double-precision%29))
  (Variables|Default|SetCurrentAgression (Math|Float|Clamp(Float) (- (Variables|Default|GetCurrentAgression) SubtractedAgression) (Variables|Default|GetMinAgression) (Variables|Default|GetMaxAgression))))