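; BPC_Hunger is a component that stores a hunger value for the actor that owns it.
; It exposes functions to read, add to and subtract from CurrentHunger, clamping each change between MinHunger and MaxHunger.
; The event graph is empty, so hunger changes only when other code calls these functions.
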(event EventBeginPlay)

(event EventTick
  (params (DeltaSeconds :type Float%20%28single-precision%29)))

(fn GetHunger
  (return (Variables|Default|GetCurrentHunger)))

(fn AddHunger
  (params (AddedHunger :type Float%20%28double-precision%29))
  (Variables|Default|SetCurrentHunger (Math|Float|Clamp(Float) (+ AddedHunger (Variables|Default|GetCurrentHunger)) (Variables|Default|GetMinHunger) (Variables|Default|GetMaxHunger)))
  (return))

(fn SubtractHunger
  (params (SubtractedHunger :type Float%20%28double-precision%29))
  (Variables|Default|SetCurrentHunger (Math|Float|Clamp(Float) (- (Variables|Default|GetCurrentHunger) SubtractedHunger) (Variables|Default|GetMinHunger) (Variables|Default|GetMaxHunger))))