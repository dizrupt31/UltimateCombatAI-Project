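; BPC_Gas is a Blueprint component that stores a gas resource value for its owner.
; It exposes a getter plus add and subtract functions, each clamping the current amount between minimum and maximum limits.
; It runs no BeginPlay or Tick logic, so the value changes only when other code calls those functions.
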(event EventBeginPlay)

(event EventTick
  (params (DeltaSeconds :type Float%20%28single-precision%29)))

(fn GetGas
  (return (Variables|Default|GetCurrentGas)))

(fn AddGas
  (params (AddedGas :type Float%20%28double-precision%29))
  (Variables|Default|SetCurrentGas (Math|Float|Clamp(Float) (+ AddedGas (Variables|Default|GetCurrentGas)) (Variables|Default|GetMinGas) (Variables|Default|GetMaxGas)))
  (return))

(fn SubtractGas
  (params (SubtractedGas :type Float%20%28double-precision%29))
  (Variables|Default|SetCurrentGas (Math|Float|Clamp(Float) (- (Variables|Default|GetCurrentGas) SubtractedGas) (Variables|Default|GetMinGas) (Variables|Default|GetMaxGas))))